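; Game mode for the mission level that tracks connected player controllers and provides player spawning.
; PostLogin and controller swaps add to the AllPCs list, while logout removes exiting BP_PC_Mission controllers.
; SpawnPlayer destroys the controller's current pawn, then spawns and possesses a BP_ThirdPersonCharacter at a randomly chosen PlayerStart.
; Nothing in this Blueprint calls SpawnPlayer itself.
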(event EventPostLogin
  (params (NewPlayer :type Player%20Controller%20Object%20Reference))
  ;[0.03122 0.06354 0.0436] On connection
  (Utilities|Array|Add (Variables|Default|GetAll%20PC's) NewPlayer))

(event EventOnSwapPlayerControllers
  (params (OldPC :type Player%20Controller%20Object%20Reference) (NewPC :type Player%20Controller%20Object%20Reference))
  ;[0.03122 0.06354 0.0436] On connection
  (Utilities|Array|Add (Variables|Default|GetAll%20PC's) NewPC))

(event EventOnLogout
  (params (ExitingController :type Controller%20Object%20Reference))
  ;[0.03122 0.06354 0.0436] On Disconnect
  (bind _asbp_pc_mission (Utilities|Casting|CastToBP_PC_Mission ExitingController))
  (Utilities|Array|RemoveItem (Variables|Default|GetAll%20PC's) _asbp_pc_mission))

(fn ConstructionScript)

(fn FindRandomPlayerstart
  (bind _outactors (Actor|GetAllActorsOfClass "/Script/Engine.PlayerStart"))
  (return (Transformation|GetActorTransform (Utilities|Array|Get(acopy) _outactors (Math|Random|RandomIntegerinRange 0 (- (Utilities|Array|Length _outactors) 1))))))

(fn SpawnPlayer
  (params (playerController :type Player%20Controller%20Object%20Reference))
  (bind _returnvalue (Pawn|GetControlledPawn playerController))
  (Utilities|IsValid _returnvalue
    (:Is%20Valid
      (Actor|DestroyActor _returnvalue))
    (:Is%20Not%20Valid
      _))
  (bind _returnvalue_2 (Game|SpawnActorfromClass "/Game/Blueprints/BP_ThirdPersonCharacter.BP_ThirdPersonCharacter_C" (Spawning|FindRandomPlayerstart) "Undefined" "MultiplyWithRoot" 0 0))
  (Pawn|Possess playerController _returnvalue_2))
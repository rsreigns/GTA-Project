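; Player controller for a mission that requests its player's spawn and gives access to the HUD options.
; On BeginPlay, the local controller calls a spawn event that asks GM_MissionGameMode to spawn its player.
; It then fetches the HUD through a GetBPHUD node with a Success callback and caches the reference.
; The Home key toggles the options on that HUD.
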(event Custom|SR_SpawnEvent
  (bind _asgm_mission_game_mode (Utilities|Casting|CastToGM_MissionGameMode (Game|GetGameMode)))
  (Default|SpawnPlayer _asgm_mission_game_mode self))

(event EventBeginPlay
  (if (Pawn|IsLocalPlayerController)
    (CallFunction|SRSpawnEvent)
    (bind _asbp_hud (Utilities|GetBPHUD 1e+01)
      (:Success
        (Variables|Default|SetrefHUD _asbp_hud)))))

(event Input|KeyboardEvents|Home
  (params (Key :type Key%20Structure :default "None"))
  (:Pressed
    (Default|ToggleOptions (Variables|Default|GetrefHUD))))

(fn ConstructionScript)
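; AI controller for civilian NPCs that starts their blackboard and behavior tree on BeginPlay.
; BeginPlay also calls a Timer event, which writes a random reachable point around the RefClass actor to Location and that actor to Player.
; The event schedules itself on a timer, then immediately calls clear on a timer handle.
; The SetRandomLocation function only zeroes CurrentLocation.
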(event Custom|timer
  (bind _blackboard (Variables|Default|GetBlackboard))
  ;[1 1 1] Timer
  (Utilities|Time|SetTimerbyEvent (delegate Custom|timer) 5.0 false 2.0)
  (Utilities|Time|ClearandInvalidateTimerbyHandle (Variables|Default|GetHandle))
  ;[1 1 1] Set Random Location
  (bind _returnvalue (Actor|GetActorOfClass (Variables|Default|GetrefClass)))
  (AI|Components|Blackboard|SetValueasVector _blackboard (Variables|Default|GetLocation) (.RandomLocation (AI|Navigation|GetRandomReachablePointinRadius (Transformation|GetActorLocation _returnvalue) 5e+03 0 0)))
  (AI|Components|Blackboard|SetValueasObject _blackboard (Variables|Default|GetPlayer) _returnvalue))

(event EventBeginPlay
  ;[1 1 1] Call Behavior tree
  (Class|AIController|UseBlackboard "/Game/Blueprints/Civillian_AI/BB_CivilBlackboard.BB_CivilBlackboard")
  (AI|RunBehaviorTree "/Game/Blueprints/Civillian_AI/BT_CivilBehavior.BT_CivilBehavior")
  (CallFunction|Timer))

(fn ConstructionScript)

(fn SetRandomLocation
  (Variables|Default|SetcurrentLocation "0, 0, 0"))
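; Player controller for driving a wheeled vehicle in the open world, handling input setup and the vehicle HUD.
; On BeginPlay and on Possess, it adds the vehicle input mapping context, creates the WB_VehicleUI widget and caches the controlled pawn's vehicle movement component.
; Each Tick feeds that component's forward speed and current gear to the HUD.
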(event EventBeginPlay
  (Development|PrintString "in the  vehicle" true true "(R=0.000000,G=0.660000,B=1.000000,A=1.000000)" 15.0)
  (Input|AddMappingContext (PlayerController|LocalPlayerSubsystems|GetEnhancedInputLocalPlayerSubsystem) "/Game/Blueprints/EnhancedActionBlueprints/Vehicle4/IMC_Vehicle4.IMC_Vehicle4" 0 "(bIgnoreAllPressedKeysUntilRelease=True,bForceImmediately=False,bNotifyUserSettings=False)") ; Adding the Input Mapping Context needed to trigger the proper Input Actions.
  (bind _returnvalue (UserInterface|CreateWidget "/Game/Blueprints/widgets/WB_VehicleUI.WB_VehicleUI_C" self))
  (bind _output_get (Variables|Default|SetVehicleHud _returnvalue))
  (UserInterface|Viewport|AddtoViewport _output_get 0)
  (bind _aswheeled_vehicle_pawn (Utilities|Casting|CastToWheeledVehiclePawn (Pawn|GetControlledPawn)))
  (Variables|Default|SetVehicle%20Movement%20Component (Variables|/Script/ChaosVehicles.WheeledVehiclePawn|GetVehicleMovementComponent _aswheeled_vehicle_pawn)))

(event EventTick
  (params (DeltaSeconds :type Float%20%28single-precision%29))
  (Default|UpdateSpeed (Variables|Default|GetVehicleHud) (Vehicle|GetForwardSpeed (Variables|Default|GetVehicle%20Movement%20Component)))
  (Default|UpdateGear (Variables|Default|GetVehicleHud) (Class|ChaosVehicleMovementComponent|GetCurrentGear (Variables|Default|GetVehicle%20Movement%20Component))))

(event EventPossess
  (params (PossessedPawn :type Pawn%20Object%20Reference))
  (Input|AddMappingContext (PlayerController|LocalPlayerSubsystems|GetEnhancedInputLocalPlayerSubsystem) "/Game/Blueprints/EnhancedActionBlueprints/Vehicle4/IMC_Vehicle4.IMC_Vehicle4" 0 "(bIgnoreAllPressedKeysUntilRelease=True,bForceImmediately=False,bNotifyUserSettings=False)") ; Adding the Input Mapping Context needed to trigger the proper Input Actions.
  (bind _returnvalue (UserInterface|CreateWidget "/Game/Blueprints/widgets/WB_VehicleUI.WB_VehicleUI_C" self))
  (bind _output_get (Variables|Default|SetVehicleHud _returnvalue))
  (UserInterface|Viewport|AddtoViewport _output_get 0)
  (bind _aswheeled_vehicle_pawn (Utilities|Casting|CastToWheeledVehiclePawn (Pawn|GetControlledPawn)))
  (Variables|Default|SetVehicle%20Movement%20Component (Variables|/Script/ChaosVehicles.WheeledVehiclePawn|GetVehicleMovementComponent _aswheeled_vehicle_pawn)))

(fn ConstructionScript)
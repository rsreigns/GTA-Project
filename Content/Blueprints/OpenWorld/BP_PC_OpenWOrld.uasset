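; Player controller for the open world mode that requests the player's spawn and handles the options menu toggle.
; On BeginPlay, the local controller fires SR_SpawnEvent, which asks GM_OpenWorld to spawn its player, then caches the HUD through GetBPHUD.
; The Home key toggles the HUD options, with a separate FlipFlop alternating between cursor with UI-only input and hidden cursor with game-only input.
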(event Custom|SR_SpawnEvent
  (bind _asgm_open_world (Utilities|Casting|CastToGM_OpenWorld (Game|GetGameMode)))
  (Default|SpawnPlayer _asgm_open_world self))

(event EventBeginPlay
  (if (Pawn|IsLocalPlayerController)
    (CallFunction|SRSpawnEvent)
    (bind _asbp_hud (Utilities|GetBPHUD 1e+01)
      (:Success
        (Variables|Default|SetrefHUD _asbp_hud)))))

(event Input|KeyboardEvents|Home
  (params (Key :type Key%20Structure :default "None"))
  (bind _returnvalue (Game|GetPlayerController 0))
  (:Pressed
    (Default|ToggleOptions (Variables|Default|GetrefHUD))
    (Utilities|FlowControl|FlipFlop
      (:A
        (Variables|Default|SetbShowMouseCursor true)
        (Input|SetInputModeUIOnly _returnvalue 0 "DoNotLock" false))
      (:B
        (Variables|Default|SetbShowMouseCursor false)
        (Input|SetInputModeGameOnly _returnvalue false)))))

(fn ConstructionScript)
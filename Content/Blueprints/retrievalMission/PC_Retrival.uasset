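; Player controller for the retrieval mission that requests player spawning and toggles the options menu.
; On BeginPlay, the local controller calls SR_SpawnEvent, which has GM_Retrieval spawn the player, then caches the HUD through GetBPHUD's success callback.
; The Home key toggles HUD options and uses a FlipFlop to alternate between UI-only input with a visible cursor and game-only input with it hidden.
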(event Custom|SR_SpawnEvent
  (bind _asgm_retrieval (Utilities|Casting|CastToGM_Retrieval (Game|GetGameMode)))
  (Default|SpawnPlayer _asgm_retrieval self))

(event EventBeginPlay
  (if (Pawn|IsLocalPlayerController)
    (CallFunction|SRSpawnEvent)
    (bind _asbp_hud (Utilities|GetBPHUD 1e+01)
      (:Success
        (Variables|Default|SetrefHUD _asbp_hud)))))

(event EventTick
  (params (DeltaSeconds :type Float%20%28single-precision%29)))

(event Input|KeyboardEvents|Home
  (params (Key :type Key%20Structure :default "None"))
  (bind _returnvalue (Game|GetPlayerController 0))
  (:Pressed
    (Default|ToggleOptions (Variables|Default|GetrefHUD))
    (Development|PrintString "toggle options")
    (Utilities|FlowControl|FlipFlop
      (:A
        (Variables|Default|SetbShowMouseCursor true)
        (Input|SetInputModeUIOnly _returnvalue 0 "DoNotLock" false))
      (:B
        (Variables|Default|SetbShowMouseCursor false)
        (Input|SetInputModeGameOnly _returnvalue false)
        (Development|PrintString "toggle off")))))

(fn ConstructionScript)
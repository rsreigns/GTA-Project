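; Game mode for the retrieval mission that tracks connected player controllers and provides player spawning.
; PostLogin and seamless controller swaps add controllers to AllPCs, while logout removes those that cast to PC_Retrival.
; SpawnPlayer, not called within this Blueprint, destroys any existing pawn, spawns a BP_FirstPersonOnly at a random PlayerStart and possesses it.
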(event EventPostLogin
  (params (NewPlayer :type Player%20Controller%20Object%20Reference))
  ;[0.03122 0.06354 0.0436] On connection
  (Utilities|Array|Add (Variables|Default|GetallPCs) NewPlayer))

(event EventOnSwapPlayerControllers
  (params (OldPC :type Player%20Controller%20Object%20Reference) (NewPC :type Player%20Controller%20Object%20Reference))
  ;[0.03122 0.06354 0.0436] On connection
  (Utilities|Array|Add (Variables|Default|GetallPCs) NewPC))

(event EventOnLogout
  (params (ExitingController :type Controller%20Object%20Reference))
  ;[0.03719 0.09687 0.08146] On disconnect
  (bind _aspc_retrival (Utilities|Casting|CastToPC_Retrival ExitingController))
  (Utilities|Array|RemoveItem (Variables|Default|GetallPCs) _aspc_retrival))

(fn ConstructionScript)

(fn FindRandomPlayerstart
  (bind _outactors (Actor|GetAllActorsOfClass "/Script/Engine.PlayerStart"))
  (return (Transformation|GetActorTransform (Utilities|Array|Get(acopy) _outactors (Math|Random|RandomIntegerinRange 0 (- (Utilities|Array|Length _outactors) 1))))))

(fn SpawnPlayer
  (params (PlayerController :type Player%20Controller%20Object%20Reference))
  (bind _returnvalue (Pawn|GetControlledPawn PlayerController))
  (Utilities|IsValid _returnvalue
    (:Is%20Valid
      (Actor|DestroyActor _returnvalue))
    (:Is%20Not%20Valid
      _))
  (bind _returnvalue_2 (CallFunction|FindRandomPlayerstart))
  (bind _returnvalue_3 (Game|SpawnActorfromClass "/Game/Blueprints/retrievalMission/BP_FirstPersonOnly.BP_FirstPersonOnly_C" _returnvalue_2 "Undefined" "MultiplyWithRoot" 0 0))
  (Pawn|Possess PlayerController _returnvalue_3)
  (return))